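; Internal rune scheduler that steps a scheduled rune config index based on the state of the active rune task.
; ReceiveScheduledRuneConfig advances the index with modulo wrap on success, resets it to zero on failure and leaves it unchanged while running or on hold.
; It returns false only for a held task, and true otherwise, including when no valid task exists.
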(fn ReceiveScheduledRuneConfig
  (params (activeRuneTask :type Rune%20Task%20Object%20Reference))
  (Utilities|IsValid activeRuneTask
    (:Is%20Valid
      (switch Utilities|FlowControl|Switch|SwitchonERuneTaskValue (Class|RuneTask|GetTaskValue activeRuneTask)
        (:SUCCESS
          (bind _result (Math|Integer|IncrementInt (Variables|Default|GetscheduledRuneConfigIndex))
            (:%20%20
              (Variables|Default|SetscheduledRuneConfigIndex (Math|Integer|%(Integer) _result (Variables|Default|GetmaxRuneConfigIndex))))))
        (:FAILURE
          (Variables|Default|SetscheduledRuneConfigIndex 0))
        (:RUNNING
          _)
        (:HOLD
          (return false)))
      (return true))
    (:Is%20Not%20Valid
      (return true))))