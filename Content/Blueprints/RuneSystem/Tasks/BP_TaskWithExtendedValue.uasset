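; Rune system task that reports a multi-state evaluation for a rune's progress: held, failed, succeeded or reset.
; On Configure it binds to each rune behaviour's activate and tangible-agent-spawn events, and to the applied event of effects of class EffectToBeApplied.
; Activation sets SECOND (hold), agent destruction sets THIRD (fail) unless already FOURTH, and an applied effect sets FOURTH (success).
; PostEvaluationUpdate returns either end state to FIRST.
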(event Custom|TaskSuccess
  (params (actor :type Actor%20Object%20Reference))
  (Class|ExtendedRuneTask|SetTaskEvaluationExtended "FOURTH"))

(event Custom|OnTanngibleAgentSpawn
  (params (agent :type Rune%20Tangible%20Agent%20Object%20Reference))
  (Game|BindEventtoOnDestroyed agent (delegate Custom|TaskFail)))

(event Custom|TaskFail
  (params (DestroyedActor :type Actor%20Object%20Reference))
  (if (Utilities|Enum|NotEqual(Enum) (Class|ExtendedRuneTask|GetTaskEvaluationExtended) "FOURTH")
    (Class|ExtendedRuneTask|SetTaskEvaluationExtended "THIRD")))

(event Custom|TaskHold
  (Class|ExtendedRuneTask|SetTaskEvaluationExtended "SECOND"))

(event EventPostEvaluationUpdate
  (bind _returnvalue (Class|ExtendedRuneTask|GetTaskEvaluationExtended))
  (if (or (Utilities|Enum|Equal(Enum) _returnvalue "THIRD") (Utilities|Enum|Equal(Enum) _returnvalue "FOURTH"))
    (Class|ExtendedRuneTask|SetTaskEvaluationExtended "FIRST")))

(event EventConfigure
  (params (runeConfiguration :type Rune%20Configuration%20Structure%20%28by%20ref%29))
  (for _array_element (.runeBehavioursWithEffects (Utilities|Struct|BreakRuneConfiguration runeConfiguration))
    (Utilities|FlowControl|Sequence
      (:then_0
        (EventDispatchers|BindEventtoOnBehaviourActivate (.runebehaviour _array_element) (delegate Custom|TaskHold)))
      (:then_1
        (EventDispatchers|BindEventtoOnTangibleAgentSpawnEnd (.runebehaviour _array_element) (delegate Custom|OnTanngibleAgentSpawn)))
      (:then_2
        (for _array_element_2 (.runeeffects _array_element)
          (if (Class|GameplayStatics|ObjectIsA _array_element_2 (Variables|Default|GetEffectToBeApplied))
            (EventDispatchers|BindEventtoOnEffectApplied _array_element_2 (delegate Custom|TaskSuccess))))))))