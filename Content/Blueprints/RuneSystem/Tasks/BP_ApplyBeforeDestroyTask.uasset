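; A rune system task that succeeds if a chosen effect class is applied before a rune's spawned tangible agent is destroyed.
; On configuration it binds to each rune behaviour's activation and agent spawn end, plus applied events of matching effects.
; Activation sets the task to hold, effect application sets success, and agent destruction sets failure unless already successful.
; After evaluation, success or failure resets to running.
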(event Custom|TaskSuccess
  (params (actor :type Actor%20Object%20Reference))
  (Class|RuneTask|SetTaskValue "SUCCESS"))

(event Custom|OnTanngibleAgentSpawn
  (params (agent :type Rune%20Tangible%20Agent%20Object%20Reference))
  (Game|BindEventtoOnDestroyed agent (delegate Custom|TaskFail)))

(event Custom|TaskFail
  (params (DestroyedActor :type Actor%20Object%20Reference))
  (if (Utilities|Enum|NotEqual(Enum) (Class|RuneTask|GetTaskValue) "SUCCESS")
    (Class|RuneTask|SetTaskValue "FAILURE")))

(event Custom|TaskHold
  (Class|RuneTask|SetTaskValue "HOLD"))

(event EventPostEvaluationUpdate
  (bind _returnvalue (Class|RuneTask|GetTaskValue))
  (if (or (Utilities|Enum|Equal(Enum) _returnvalue "SUCCESS") (Utilities|Enum|Equal(Enum) _returnvalue "FAILURE"))
    (Class|RuneTask|SetTaskValue "RUNNING")))

(event EventConfigure
  (params (runeConfiguration :type Rune%20Configuration%20Structure%20%28by%20ref%29))
  (for _array_element (.runeBehavioursWithEffects (Utilities|Struct|BreakRuneConfiguration runeConfiguration))
    (Utilities|FlowControl|Sequence
      (:then_0
        (EventDispatchers|BindEventtoOnBehaviourActivate (.runebehaviour _array_element) (delegate Custom|TaskHold)))
      (:then_1
        (EventDispatchers|BindEventtoOnTangibleAgentSpawnEnd (.runebehaviour _array_element) (delegate Custom|OnTanngibleAgentSpawn)))
      (:then_2
        (for _array_element_2 (.runeeffects _array_element)
          (if (Class|GameplayStatics|ObjectIsA _array_element_2 (Variables|Default|GetEffectToBeApplied))
            (EventDispatchers|BindEventtoOnEffectApplied _array_element_2 (delegate Custom|TaskSuccess))))))))