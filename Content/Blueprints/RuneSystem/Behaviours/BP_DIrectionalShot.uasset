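; BP_DIrectionalShot is a rune behaviour that fires an agent in the rune owner's aim direction when activated.
; It reads the rune input from a valid owner and spawns a tangible agent from AgentTemplate, rotated to face the aim.
; The spawn point is the input origin pushed along the aim by Offset X and raised by Offset Z, leaving Offset Y unused.
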(event EventBeginPlay)

(event EventTick
  (params (DeltaSeconds :type Float%20%28single-precision%29)))

(event EventActivateBehaviour
  (bind _offset (Variables|Default|GetOffset))
  (bind _runeowner (Variables|Default|GetruneOwner))
  (Utilities|IsValid (Utilities|ToObject(Interface) _runeowner)
    (:Is%20Valid
      (bind _returnvalue (Class|RuneCompatible|GetRuneInput _runeowner))
      (Class|RuneBehaviour|SpawnTangibleAgentwithTemplate (Variables|Default|GetAgent%20Template) (Math|Transform|MakeTransform (+ (.originLocation (Utilities|Struct|BreakRuneInput _returnvalue)) (* (.aimDirection (Utilities|Struct|BreakRuneInput _returnvalue)) (.x _offset)) (Math|Vector|MakeVector 0.0 0.0 (.z _offset))) (Math|Conversions|RotationFromXVector (.aimDirection (Utilities|Struct|BreakRuneInput _returnvalue))))))))