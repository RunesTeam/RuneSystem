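; BP_InstantCast is a cast state machine for the rune system that fires instantly on press.
; On Init it constructs Idle and Pressed state objects, sets Idle as the entry state and binds their enter and tick callbacks.
; Idle switches to Pressed when IsPressed is true, entering Pressed activates every behaviour slot once, and Pressed returns to Idle on release.
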(event EventBeginPlay)

(event EventTick
  (params (DeltaSeconds :type Float%20%28single-precision%29)))

(event EventInit
  (Utilities|FlowControl|Sequence
    (:then_0
      (bind _returnvalue (Game|ConstructObjectfromClass self (Variables|Default|GetState%20Class%20Reference)))
      (bind _output_get (Variables|Default|Setidle _returnvalue))
      (Class|RuneCastStateMachine|SetEntryState _output_get)
      (bind _returnvalue_2 (Game|ConstructObjectfromClass self (Variables|Default|GetState%20Class%20Reference)))
      (Variables|Default|Setpressed _returnvalue_2))
    (:then_1
      (EventDispatchers|BindEventtoOnTick (Variables|Default|Getidle) (EventDispatchers|CreateEvent :!event IdleTick))
      (EventDispatchers|BindEventtoOnEnter (Variables|Default|Getpressed) (EventDispatchers|CreateEvent :!event PressedonEnter))
      (EventDispatchers|BindEventtoOnTick (Variables|Default|Getpressed) (EventDispatchers|CreateEvent :!event PressedTick)))))

(fn IdleTick
  (params (deltaTime :type Float%20%28single-precision%29))
  (if (Variables|Default|GetisPressed)
    (Class|RuneCastStateMachine|ChangeState (Variables|Default|Getpressed))))

(fn PressedonEnter
  (for (_ _array_index) (Class|RuneCastStateMachine|GetBehaviourSlots)
    (Class|RuneCastStateMachine|ActivateBehaviourSlot _array_index)))

(fn PressedTick
  (params (deltaTime :type Float%20%28single-precision%29))
  (if (not (Variables|Default|GetisPressed))
    (Class|RuneCastStateMachine|ChangeState (Variables|Default|Getidle))))